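; BP_SliceKnife is a cooking-simulator knife that cuts procedural meshes while the player TestCharacter's Slice flag is set.
; When BaseMesh begins overlapping, a DoOnce stores the touched ProceduralMeshComponent.
; When overlap ends, it resets that latch and slices the stored mesh along a plane from the Point component's location and forward vector.
; The slice creates a capped other half with physics simulation enabled; an impulse node is left unconnected.
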(event `self.baseMesh.OnComponentBeginOverlap`
  (params (OverlappedComponent :type "PrimitiveComponent Object Reference") (OtherActor :type "Actor Object Reference") (OtherComp :type "PrimitiveComponent Object Reference") (OtherBodyIndex :type Integer) (bFromSweep :type Boolean) (SweepResult :type "HitResult Structure (by ref)"))
  (if (`TestCharacter.bSlice` (cast `TestCharacter` (`GameplayStatics.GetPlayerPawn` 0) :!pure true))
    (`/Engine/EditorBlueprintResources/StandardMacros.DoOnce` false :!label _label
      (:`Completed`
        (bind _asprocedural_mesh_component (cast `ProceduralMeshComponent` OtherComp))))))

(event `self.baseMesh.OnComponentEndOverlap`
  (params (OverlappedComponent :type "PrimitiveComponent Object Reference") (OtherActor :type "Actor Object Reference") (OtherComp :type "PrimitiveComponent Object Reference") (OtherBodyIndex :type Integer))
  (bind _point (`self.point`))
  (if (`TestCharacter.bSlice` (cast `TestCharacter` (`GameplayStatics.GetPlayerPawn` 0) :!pure true))
    (`|ExecutionSequence`
      (:`then_0`
        (goto _label :!via `Reset`))
      (:`then_1`
        (`/Engine/EditorBlueprintResources/StandardMacros.IsValid` (stale `self.baseMesh.OnComponentBeginOverlap` _asprocedural_mesh_component)
          (:`Is Valid`
            _)
          (:`Is Not Valid`
            _))
        (bind _outotherhalfprocmesh (`KismetProceduralMeshLibrary.SliceProceduralMesh` (stale `self.baseMesh.OnComponentBeginOverlap` _asprocedural_mesh_component) (`SceneComponent.K2_GetComponentLocation` _point) (`SceneComponent.GetForwardVector` _point) true "CreateNewSectionForCap" "/DatasmithContent/Materials/AliasReference.AliasReference"))
        (`PrimitiveComponent.SetSimulatePhysics` _outotherhalfprocmesh true)))))

(fn `UserConstructionScript`)