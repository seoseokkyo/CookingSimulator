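; BP_SliceMesh is a test actor for runtime mesh slicing in the cooking simulator.
; Construction copies the Cube static mesh into a procedural mesh with collision.
; Pressing 6 slices it along a plane offset from the player pawn by the actor's forward vector, which also serves as the normal.
; The cut gets a capped section, and the returned half simulates physics and receives an impulse.
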(event `self.ReceiveBeginPlay`
  (`self.EnableInput` (`GameplayStatics.GetPlayerController` 0)))

(event `Key|Six`
  (params (Key :type "Key Structure"))
  (:`Pressed`
    (`KismetSystemLibrary.PrintString` "Hello")
    (bind _outotherhalfprocmesh (`KismetProceduralMeshLibrary.SliceProceduralMesh` (`self.ProceduralMesh`) (+ (`self.K2_GetActorLocation` (`GameplayStatics.GetPlayerPawn` 0)) (* (`self.GetActorForwardVector`) 100.0)) (`self.GetActorForwardVector`) true "CreateNewSectionForCap" "/DatasmithContent/Materials/AliasReference.AliasReference"))
    (`PrimitiveComponent.SetSimulatePhysics` _outotherhalfprocmesh true)
    (`PrimitiveComponent.AddImpulse` _outotherhalfprocmesh (300.0 300.0 300.0) "None" true)))

(fn `UserConstructionScript`
  (`KismetProceduralMeshLibrary.CopyProceduralMeshFromStaticMeshComponent` (`self.Cube`) 0 (`self.ProceduralMesh`) true))